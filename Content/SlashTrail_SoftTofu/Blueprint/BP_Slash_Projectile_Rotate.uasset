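; BP_Slash_Projectile_Rotate is a slash projectile actor with a sword mesh that spins every tick and an NSSlash effect.
; It plays a sound on spawn and destroys itself after a short lifetime.
; A Box hit spawns a scaled-down impact effect and sound at the hit point, then staggers cleanup: effect deactivation and sword hiding after a brief delay, actor destruction later.
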(event `self.ReceiveTick`
  (params (DeltaSeconds :type "Float (single-precision)"))
  (`SceneComponent.K2_AddWorldRotation` (`self.SK_Sword`) (`self.Delta Rotation`) false false))

(event `self.ReceiveBeginPlay`
  (`GameplayStatics.PlaySoundAtLocation` (`self.Sound`) (`self.K2_GetActorLocation`) (struct) 1.0 1.0 0.0 null null null null)
  (`KismetSystemLibrary.Delay` 3.0)
  (`self.K2_DestroyActor`))

(event `self.Box.OnComponentHit`
  (params (HitComponent :type "PrimitiveComponent Object Reference") (OtherActor :type "Actor Object Reference") (OtherComp :type "PrimitiveComponent Object Reference") (NormalImpulse :type "Vector Structure") (Hit :type "HitResult Structure (by ref)"))
  (`NiagaraFunctionLibrary.SpawnSystemAtLocation` (`self.Hit Particle`) Hit_Location (struct) (0.5 0.5 0.5))
  (`GameplayStatics.PlaySoundAtLocation` (`self.Hit_Sound`) Hit_Location (struct) 1.0 1.0 0.0 null null null null)
  (`KismetSystemLibrary.Delay` 0.2)
  (`ActorComponent.Deactivate` (`self.NS_Slash`))
  (`SceneComponent.SetHiddenInGame` (`self.SK_Sword`) true false)
  (`KismetSystemLibrary.Delay` 1.0)
  (`self.K2_DestroyActor`))

(fn `UserConstructionScript`)